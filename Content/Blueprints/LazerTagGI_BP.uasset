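; LazerTagGI_BP is the game instance for a laser tag game, handling online session hosting, joining and player naming.
; HostGame creates an Advanced Sessions session with optional LAN and opens the Lobby map as a listen server, clearing HostSuccessful on failure.
; JoinGame joins a given search result, sharing the network error handler's red debug print on failure.
; SetName stores the local player's Steam nickname in PNAME.
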(event Custom|SetName
  ;[1 1 1] Gets steam name for this player
  (Variables|Default|SetPNAME (Class|AdvancedIdentityLibrary|GetPlayerNickname (Class|AdvancedSessionsLibrary|GetUniqueNetID (Game|GetPlayerController 0)))))

(event Custom|JoinGame
  (params (SearchResult :type Blueprint%20Session%20Result%20Structure%20%28by%20ref%29))
  (|JoinSession (Game|GetPlayerController 0) SearchResult
    (:OnFailure
      (Development|PrintString (Utilities|String|EnumtoString (stale EventHandleNetworkError FailureType)) true true "(R=1.000000,G=0.000000,B=0.024691,A=1.000000)"))))

(event Custom|HostGame
  (params (bUseLAN :type Boolean))
  (|AdvancedSession 0 (Game|GetPlayerController 0) 4 4 bUseLAN true false true true false false false true
    (:OnSuccess
      (Game|OpenLevel(byName) "Lobby" true "Listen"))
    (:OnFailure
      (Variables|Default|SetbHostSuccessful false)
      (Development|PrintString (Utilities|String|EnumtoString (stale EventHandleNetworkError FailureType)) true true "(R=1.000000,G=0.000000,B=0.024691,A=1.000000)"))))

(event EventHandleNetworkError
  (params (FailureType :type ENetworkFailure%20Enum :default "NetDriverAlreadyExists") (bIsServer :type Boolean))
  (Development|PrintString (Utilities|String|EnumtoString FailureType) true true "(R=1.000000,G=0.000000,B=0.024691,A=1.000000)"))