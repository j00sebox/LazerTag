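; Player state for the laser tag game that carries each player's name and reacts to score and lobby roster changes.
; On BeginPlay it caches the game instance and game state, then passes the stored name through server and client set-name events so other players see it.
; Leaderboard updates end the game at the score limit or re-sort players.
; A player-array OnRep rebuilds the lobby screen list, and another event destroys the session.
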(event Custom|AddPlayersToLobby
  (bind _aslobby_pc (Utilities|Casting|CastToLobby_PC (Game|GetPlayerController 0)))
  (Utilities|IsValid (Variables|/Game/Lobby/Lobby_PC.Lobby_PC_C|GetLobbyScreenRef _aslobby_pc)
    (:Is%20Valid
      (Default|Clear (Variables|/Game/Lobby/Lobby_PC.Lobby_PC_C|GetLobbyScreenRef _aslobby_pc))
      (bind _aslobby_game_state (Utilities|Casting|CastToLobby_GameState (Game|GetGameState)))
      (for _array_element (Variables|/Script/Engine.GameStateBase|GetPlayerArray _aslobby_game_state)
        (bind _aspstate_bp (Utilities|Casting|CastToPState_BP _array_element))
        (Default|AddPlayer (Variables|/Game/Lobby/Lobby_PC.Lobby_PC_C|GetLobbyScreenRef _aslobby_pc) (Variables|/Script/LazerTag.PState|GetplayerName _aspstate_bp))))))

(event Custom|DestroyGameSession
  (|DestroySession (Game|GetPlayerController 0)))

(event Custom|GetSteamName
  ;[1 1 1] Makes sure all names are visible on all connected players
  (bind _aslazer_tag_gi_bp (Utilities|Casting|CastToLazerTagGI_BP (Game|GetGameInstance)))
  (CallFunction|ServerSetName (Variables|/Game/Blueprints/LazerTagGI_BP.LazerTagGI_BP_C|GetPNAME _aslazer_tag_gi_bp)))

(event Custom|ServerSetName
  (params (Player%20Name :type String))
  ;[1 1 1] Makes sure all names are visible on all connected players
  (bind _output_get (Variables|Default|SetplayerName Player%20Name))
  (CallFunction|ClientSetName _output_get))

(event Custom|ClientSetName
  (params (Player%20Name :type String))
  ;[1 1 1] Makes sure all names are visible on all connected players
  (Variables|Default|SetplayerName Player%20Name))

(event EventBeginPlay
  (CallFunction|GetSteamName)
  (bind _aslazer_tag_gi (Utilities|Casting|CastToLazerTag_GI (Game|GetGameInstance)))
  (Variables|Default|SetLazerTagGIRef _aslazer_tag_gi)
  (bind _aslazer_tag_game_state (Utilities|Casting|CastToLazerTag_GameState (Game|GetGameState)))
  (Variables|Default|SetAs%20Lazer%20Tag%20Game%20State _aslazer_tag_game_state))

(event EventUpdateLeaderBoardPos
  (if (>= (Class|PState|GetCurrentScore) (Class|LazerTagGI|GetScoreLimit (Variables|Default|GetLazerTagGIRef)))
    (Default|EndGame (Variables|Default|GetAs%20Lazer%20Tag%20Game%20State))
    (else
      (Default|SortPlayers (Variables|Default|GetAs%20Lazer%20Tag%20Game%20State)))))

(fn ConstructionScript)

(fn OnRepPlayerArrayChanged
  (CallFunction|AddPlayerstoLobby))