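; Game state for laser tag that holds the match countdown and a score-ranked player list.
; Each Timer call waits one second, then steps down Minutes and Seconds once, with no loop in this graph.
; At zero, EndGame travels to the Lobby level and game mode through LazerTag_GI.
; UpdateSortedPlayers copies PlayerArray and bubble-sorts it by PState_BP current score, highest first.
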(event Custom|Timer
  ;[1 0.7317 0.237] Timer
  (Utilities|FlowControl|Delay 1.0)
  (if (== (Variables|Default|GetSeconds) 0)
    (if (== (Variables|Default|GetMinutes) 0)
      (CallFunction|EndGame)
      (else
        (Variables|Default|SetSeconds 59)
        (Variables|Default|SetMinutes (- (Variables|Default|GetMinutes) 1))))
    (else
      (Variables|Default|SetSeconds (- (Variables|Default|GetSeconds) 1)))))

(event Custom|Update%20Sorted%20Players
  (Variables|Default|SetSortedPlayers (Variables|Default|GetPlayerArray))
  (CallFunction|SortPlayers))

(event Custom|SortPlayers
  (bind _sortedplayers (Variables|Default|GetSortedPlayers))
  (bind _sortedplayers_2 (Variables|Default|GetSortedPlayers))
  (bind _returnvalue (Utilities|Array|Length _sortedplayers))
  (bind _returnvalue_2 (- _returnvalue 1))
  ;[0.07 0.06 1] for (i = 0;i< n-1;i++)
  (for _index (range 0 _returnvalue_2)
    ;[0.07 0.07 1] for (j = 0; j < n - i - 1; j++)
    (for _index_2 (range 0 (- _returnvalue_2 _index))
      (bind _aspstate_bp (Utilities|Casting|CastToPState_BP (Utilities|Array|Get(acopy) _sortedplayers_2 _index_2)))
      (bind _aspstate_bp_2 (Utilities|Casting|CastToPState_BP (Utilities|Array|Get(acopy) _sortedplayers_2 (+ _index_2 1))))
      ;;[1 1 1] if arr[j] > arr[j+1] then swap
      (if (> (Class|PState|GetCurrentScore _aspstate_bp_2) (Class|PState|GetCurrentScore _aspstate_bp))
        (Utilities|Array|Swap (Variables|Default|GetSortedPlayers) _index_2 (+ _index_2 1))))))

(event Custom|SetInitialTime
  (params (Seconds :type Integer) (Minutes :type Integer))
  (Variables|Default|SetSeconds Seconds)
  (Variables|Default|SetMinutes Minutes))

(event Custom|EndGame
  (bind _aslazer_tag_gi (Utilities|Casting|CastToLazerTag_GI (Game|GetGameInstance)))
  (Class|LazerTagGI|Travel _aslazer_tag_gi "/Game/Levels/Lobby" "/Game/Lobby/Lobby_GameMode"))

(fn ConstructionScript)