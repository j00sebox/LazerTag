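; LazerTag is a game mode Blueprint that drives the match timer and player list for a laser tag game.
; On BeginPlay it caches the LazerTag game state and sets its starting time in minutes from the time limit stored in the game instance.
; It calls the game state's Timer every Tick and has it update the sorted player list on each PostLogin.
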(event EventBeginPlay
  (bind _aslazer_tag_game_state (Utilities|Casting|CastToLazerTag_GameState (Game|GetGameState)))
  (bind _output_get (Variables|Default|SetGameStateRef _aslazer_tag_game_state))
  (bind _aslazer_tag_gi (Utilities|Casting|CastToLazerTag_GI (Game|GetGameInstance)))
  (Default|SetInitialTime _output_get 0 (Class|LazerTagGI|GetTimeLimit _aslazer_tag_gi)))

(event EventTick
  (params (DeltaSeconds :type Float%20%28single-precision%29))
  (Default|Timer (Variables|Default|GetGameStateRef)))

(event EventPostLogin
  (params (NewPlayer :type Player%20Controller%20Object%20Reference))
  (bind _aslazer_tag_game_state (Utilities|Casting|CastToLazerTag_GameState (Game|GetGameState)))
  (Default|UpdateSortedPlayers _aslazer_tag_game_state))

(fn ConstructionScript)